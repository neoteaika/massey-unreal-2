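; Proximity sliding door that opens for BP_nChar_Grabber and closes when it leaves, unless Offline or OnlineLocked.
; Trigger overlaps play sounds, set the status and drive the DoorMovement timeline forward or in reverse, moving both panels through DoorDistanceProcessor.
; UpdateElectronics maps each status, including Hacking, to front/back banner text and a colour for four lights.
; Construction script applies the spawn status and caches the panels' initial positions.
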(event OnComponentBeginOverlap(DoorTest)
  (params (OverlappedComponent :type Primitive%20Component%20Object%20Reference) (OtherActor :type Actor%20Object%20Reference) (OtherComp :type Primitive%20Component%20Object%20Reference) (OtherBodyIndex :type Integer) (bFromSweep :type Boolean) (SweepResult :type Hit%20Result%20Structure%20%28by%20ref%29))
  (if (and (Utilities|Enum|NotEqual(Enum) (Variables|Default|Getstatus_door) "NewEnumerator3") (Utilities|Enum|NotEqual(Enum) (Variables|Default|Getstatus_door) "NewEnumerator1"))
    (Utilities|Casting|CastToBP_nChar_Grabber OtherActor)
    (Audio|PlaySound2D "/Engine/VREditor/Sounds/UI/Camera_Shutter.Camera_Shutter" 1.0 1.0 0.0 0 0)
    (Audio|PlaySoundatLocation "/Game/_nOrbital/snd/door/PM_FSSF_DOOR_MID_9.PM_FSSF_DOOR_MID_9" (Transformation|GetActorLocation) "0, 0, 0" 1.0 1.0 0.0 0 0 0 0)
    (Variables|Default|Setstatus_door "NewEnumerator0")
    (CallFunction|UpdateElectronics)
    (bind _doortrack (Timeline|DoorMovement PlayFromStart)
      (:Update
        (Transformation|SetRelativeLocation (Variables|Default|GetDoorLeft) (.Door%20Left%20Location (|DoorDistanceProcessor _doortrack (Variables|Default|GetDoor%20Open%20Distance))) false false)
        (Transformation|SetRelativeLocation (Variables|Default|GetDoorRight) (.Door%20Right%20Location (|DoorDistanceProcessor _doortrack (Variables|Default|GetDoor%20Open%20Distance))) false false)))))

(event OnComponentEndOverlap(DoorTest)
  (params (OverlappedComponent :type Primitive%20Component%20Object%20Reference) (OtherActor :type Actor%20Object%20Reference) (OtherComp :type Primitive%20Component%20Object%20Reference) (OtherBodyIndex :type Integer))
  (if (and (Utilities|Enum|NotEqual(Enum) (Variables|Default|Getstatus_door) "NewEnumerator3") (Utilities|Enum|NotEqual(Enum) (Variables|Default|Getstatus_door) "NewEnumerator1"))
    (Utilities|Casting|CastToBP_nChar_Grabber OtherActor)
    (Audio|PlaySound2D "/Engine/EditorSounds/Notifications/CompileFailed.CompileFailed" 1.0 1.0 0.0 0 0)
    (Audio|PlaySoundatLocation "/Game/_nOrbital/snd/door/transition_shutter_002.transition_shutter_002" (Transformation|GetActorLocation) "0, 0, 0" 1.0 1.0 0.0 0 0 0 0)
    (Variables|Default|Setstatus_door "NewEnumerator2")
    (CallFunction|UpdateElectronics)
    (bind _doortrack (Timeline|DoorMovement ReverseFromEnd)
      (:Update
        (Transformation|SetRelativeLocation (Variables|Default|GetDoorLeft) (.Door%20Left%20Location (|DoorDistanceProcessor _doortrack (Variables|Default|GetDoor%20Open%20Distance))) false false)
        (Transformation|SetRelativeLocation (Variables|Default|GetDoorRight) (.Door%20Right%20Location (|DoorDistanceProcessor _doortrack (Variables|Default|GetDoor%20Open%20Distance))) false false)))))

(event EventBeginPlay)

(event Collision|EventActorBeginOverlap
  (params (OtherActor :type Actor%20Object%20Reference)))

(event EventTick
  (params (DeltaSeconds :type Float%20%28single-precision%29)))

(fn ConstructionScript
  (Variables|Default|Setstatus_door (Variables|Default|Getstatus_door_at_spawn))
  (CallFunction|UpdateElectronics)
  (bind _output_get (Variables|Default|SetDoor%20L%20Init%20Position (Variables|/Script/Engine.SceneComponent|GetRelativeLocation (Variables|Default|GetDoorLeft))))
  (bind _output_get_2 (Variables|Default|SetDoor%20R%20Init%20Position (Variables|/Script/Engine.SceneComponent|GetRelativeLocation (Variables|Default|GetDoorRight))))
  (Development|PrintString (Utilities|String|ToString(Vector) _output_get))
  (Development|PrintString (Utilities|String|ToString(Vector) _output_get_2)))

(fn UpdateElectronics
  (switch Utilities|FlowControl|Switch|Switchonenum_DoorState (Variables|Default|Getstatus_door)
    (:NewEnumerator0
      (Utilities|SetDoorText "OPEN"
        (:X%20Out
          (Utilities|SetDoorLights (Variables|Default|Getcolorkey_open)))))
    (:NewEnumerator1
      (Utilities|SetDoorText "LOCKED"
        (:X%20Out
          (Utilities|SetDoorLights (Variables|Default|Getcolorkey_locked)))))
    (:NewEnumerator2
      (Utilities|SetDoorText "CLOSED"
        (:X%20Out
          (Utilities|SetDoorLights (Variables|Default|Getcolorkey_closed)))))
    (:NewEnumerator3
      (Utilities|SetDoorText
        (:X%20Out
          (Utilities|SetDoorLights (Variables|Default|Getcolorkey_offline)))))
    (:NewEnumerator4
      (Utilities|SetDoorText "###"
        (:X%20Out
          (Utilities|SetDoorLights (Variables|Default|Getcolorkey_hacking)))))))