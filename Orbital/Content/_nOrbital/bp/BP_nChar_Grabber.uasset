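; BP_nChar_Grabber is a possessable character with look-driven jet effects and a scene capture feed.
; Look and turn input rotate the controller and toggle paired jet components beyond a deadzone.
; Possession overrides the audio listener, BeginPlay assigns the capture's render target, and capsule hits play a sound.
; E or left click runs a debug-drawn camera line trace, but its result drives nothing yet.
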(event OnComponentHit(CapsuleComponent)
  (params (HitComponent :type Primitive%20Component%20Object%20Reference) (OtherActor :type Actor%20Object%20Reference) (OtherComp :type Primitive%20Component%20Object%20Reference) (NormalImpulse :type Vector :default "0, 0, 0") (Hit :type Hit%20Result%20Structure%20%28by%20ref%29))
  (Audio|PlaySound2D "/Game/_nOrbital/snd/nfx/hbfx_rec1_31.hbfx_rec1_31" 0.5 1.0 0.0 0 self))

(event EventBeginPlay
  (|CallParentFunction)
  (Variables|/Script/Engine.SceneCaptureComponent2D|SetTextureTarget (Variables|Default|GetSceneCaptureComponent2D) (Variables|Default|GetTexture%20Target)))

(event Collision|EventActorBeginOverlap
  (params (OtherActor :type Actor%20Object%20Reference)))

(event EventTick
  (params (DeltaSeconds :type Float%20%28single-precision%29))
  (|CallParentFunction DeltaSeconds) ; This node is disabled and will not be called.\nDrag off pins to build functionality.
)

(event EventPossessed
  (params (NewController :type Controller%20Object%20Reference))
  (bind _returnvalue (Game|GetPlayerController 0))
  (Class|PlayerController|ClearAudioListenerOverride _returnvalue)
  (Class|PlayerController|SetAudioListenerOverride _returnvalue (Class|Actor|GetParentComponent (Game|Player|GetPlayerPawn 0)) (Transformation|GetActorLocation NewController) "0, 0, 0"))

(event Input|AxisEvents|InputAxisTurn
  (params (AxisValue :type Float%20%28single-precision%29))
  ;[1 0.5426 0.9995] Camera
  (Pawn|Input|AddControllerYawInput AxisValue))

(event Input|AxisEvents|InputAxisLookUp
  (params (AxisValue :type Float%20%28single-precision%29))
  ;[1 0.5426 0.9995] Camera
  (Pawn|Input|AddControllerPitchInput AxisValue))

(event Input|AxisEvents|InputAxisTurn
  (params (AxisValue :type Float%20%28single-precision%29))
  (bind _jetleft (Variables|Default|GetJetLeft))
  (bind _jetright (Variables|Default|GetJetRight))
  (if (and (< AxisValue 0.5) (> AxisValue -0.5))
    (Components|Activation|Deactivate _jetleft)
    (Components|Activation|Deactivate _jetright)
    (else
      (Components|Activation|Activate _jetleft true)
      (Components|Activation|Activate _jetright true))))

(event Input|AxisEvents|InputAxisLookUp
  (params (AxisValue :type Float%20%28single-precision%29))
  (bind _jetup (Variables|Default|GetJetUp))
  (bind _jetdown (Variables|Default|GetJetDown))
  (if (and (< AxisValue 0.5) (> AxisValue -0.5))
    (Components|Activation|Deactivate _jetup)
    (Components|Activation|Deactivate _jetdown)
    (else
      (Components|Activation|Activate _jetup true)
      (Components|Activation|Activate _jetdown true))))

(fn ConstructionScript
  (|CallParentFunction))

(fn Interact
  (|CallParentFunction))

(event Input|KeyboardEvents|E
  (params (Key :type Key%20Structure))
  (:Pressed
    (return)))

(event Input|MouseEvents|LeftMouseButton
  (params (Key :type Key%20Structure))
  (:Pressed
    (|Outputs) ; enters at Pressed2
  ))