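; Player character Blueprint that tracks a draining suit oxygen supply and carries early interaction scaffolding.
; Tick lowers O2 over time, prints it on screen and updates the progress bar and number in the HUD_player widget component.
; E or left mouse fires a debug-drawn camera trace, multiplying location by the forward offset, with its hit unused.
; Possession and key 5 only cast the ticker widget; typewriter and audio-listener code is disconnected.
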(event EventBeginPlay
  (|CallParentFunction) ; This node is disabled and will not be called.\nDrag off pins to build functionality.
)

(event Collision|EventActorBeginOverlap
  (params (OtherActor :type Actor%20Object%20Reference)))

(event EventPossessed
  (params (NewController :type Controller%20Object%20Reference))
  (Utilities|FlowControl|Sequence
    (:then_1
      (bind _aswbp_typetext (Utilities|Casting|CastToWBP_typetext (UserInterface|GetWidget (Variables|Default|GetWidget%20Ticker)))))))

(event EventTick
  (params (DeltaSeconds :type Float%20%28single-precision%29))
  (Utilities|FlowControl|Sequence
    (:then_0
      (bind _output_get (Variables|Default|SetO2 (- (Variables|Default|GetO2) (* DeltaSeconds 0.5))))
      (Development|PrintString (Utilities|String|Append (Utilities|String|ToString(Integer) (Class|KismetMathLibrary|FTrunc64 _output_get)) "% O2 in suit") true false "(R=1.000000,G=0.568739,B=0.149801,A=1.000000)" 1.0 "Air"))
    (:then_1
      (bind _ashud_player (Utilities|Casting|CastToHUD_player (UserInterface|GetWidget (Variables|Default|GetWidget%20Main))))
      (Progress|SetPercent (Variables|/Game/_nOrbital/ui/HUD_player.HUD_player_C|Getairprogress _ashud_player) (/ (Variables|Default|GetO2) 1e+02))
      (Rendering|Components|TextRender|SetText (Variables|/Game/_nOrbital/ui/HUD_player.HUD_player_C|Getairnumber _ashud_player) (Class|KismetTextLibrary|AsPercentFloat (Variables|Default|GetO2) "HalfToEven" true)))))

(event Input|KeyboardEvents|5
  (params (Key :type Key%20Structure :default "None"))
  (:Pressed
    (bind _aswbp_typetext (Utilities|Casting|CastToWBP_typetext (UserInterface|GetWidget (Variables|Default|GetWidget%20Ticker))))))

(fn ConstructionScript
  (|CallParentFunction))

(fn Interact
  (|CallParentFunction))

(event Input|KeyboardEvents|E
  (params (Key :type Key%20Structure :default "None"))
  (:Pressed
    (return)))

(event Input|MouseEvents|LeftMouseButton
  (params (Key :type Key%20Structure :default "None"))
  (:Pressed
    (|Outputs) ; enters at Pressed2
  ))