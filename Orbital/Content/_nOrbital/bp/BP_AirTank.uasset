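; Air tank pickup that refills the player character's oxygen when interacted with.
; Its Interactwith event fires a typed-text "AIR TANK" message, prints a debug string, plays a sound, then adds a fixed amount to BP_nChar_You's O2 with no clamp and destroys itself.
; The item query functions report no fracture, a single item type and no mesh.
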(event EventBeginPlay)

(event Collision|EventActorBeginOverlap
  (params (OtherActor :type Actor%20Object%20Reference)))

(event EventTick
  (params (DeltaSeconds :type Float%20%28single-precision%29)))

(event EventInteractwith
  (Default|CallTypeEvent "AIR TANK" 0.0 0.0)
  (Development|PrintString "Collected AIR TANK")
  (Audio|PlaySound2D "/Engine/EditorSounds/GamePreview/EndSimulate.EndSimulate" 1.0 1.0 0.0 0 0)
  (bind _asbp_n_char_you (Utilities|Casting|CastToBP_nChar_You (Game|Player|GetPlayerPawn 0)))
  (Variables|/Game/_nOrbital/bp/BP_nChar_You.BP_nChar_You_C|SetO2 _asbp_n_char_you (+ (Variables|/Game/_nOrbital/bp/BP_nChar_You.BP_nChar_You_C|GetO2 _asbp_n_char_you) 25.0))
  (Actor|DestroyActor))

(fn ConstructionScript)

(fn GetFractureBool
  (return false))

(fn GetItemType
  (return "NewEnumerator0"))

(fn GetMesh
  (return 0))