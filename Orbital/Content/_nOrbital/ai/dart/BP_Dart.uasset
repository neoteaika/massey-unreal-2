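; BP_Dart is an AI dart projectile that homes in on the player character.
; On BeginPlay and on a looping one-second timer, it casts the player to BP_nChar_Grabber and sets that character's mesh as the ProjectileMovement homing target.
; An AIPerception component only prints a debug message on perception updates and does not affect the homing.
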(event OnPerceptionUpdated(AIPerception)
  (params (UpdatedActors :type Array%20of%20Actor%20Object%20References))
  (Development|PrintString "Dart spotted movement"))

(event Custom|HomeOnPlayer
  (CallFunction|HomingonPlayer))

(event EventBeginPlay
  (CallFunction|HomingonPlayer)
  (Utilities|Time|SetTimerbyEvent (delegate Custom|HomeOnPlayer) 1.0 true true))

(event Collision|EventActorBeginOverlap
  (params (OtherActor :type Actor%20Object%20Reference)))

(event EventTick
  (params (DeltaSeconds :type Float%20%28single-precision%29)))

(fn ConstructionScript)

(fn HomingonPlayer
  (bind _asbp_n_char_grabber (Utilities|Casting|CastToBP_nChar_Grabber (Game|GetPlayerCharacter 0)))
  (Variables|/Script/Engine.ProjectileMovementComponent|SetHomingTargetComponent (Variables|Default|GetProjectileMovement) (Variables|/Script/Engine.Character|GetMesh _asbp_n_char_grabber)))