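; BP_WinPickUp is a win-condition pickup actor, in the JeremyPuzzle folder, that shows a victory screen when the player touches it.
; Its Collision overlap checks for the player pawn and fires once through a DoOnce.
; It then adds the UI_WinScreen widget to the viewport and destroys the SMWinItem component.
; After a short delay it removes the widget and destroys itself.
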(event OnComponentBeginOverlap(Collision)
  (params (OverlappedComponent :type Primitive%20Component%20Object%20Reference) (OtherActor :type Actor%20Object%20Reference) (OtherComp :type Primitive%20Component%20Object%20Reference) (OtherBodyIndex :type Integer) (bFromSweep :type Boolean) (SweepResult :type Hit%20Result%20Structure%20%28by%20ref%29))
  ;[1 1 1] Checks if Player
  (if (== OtherActor (Game|Player|GetPlayerPawn 0))
    ;[1 1 1] Displays You Win UI
    (Utilities|FlowControl|DoOnce false
      (:Completed
        (bind _returnvalue (UserInterface|CreateWidget "/Game/JeremyPuzzle/UI/UI_WinScreen.UI_WinScreen_C" (Game|GetPlayerController 0)))
        (UserInterface|Viewport|AddtoViewport _returnvalue 0)
        (Components|DestroyComponent (Variables|Default|GetSM_WinItem))
        (Utilities|FlowControl|Delay 3.0)
        (Widget|RemovefromParent _returnvalue)
        (Actor|DestroyActor)))))

(event EventBeginPlay)

(event Collision|EventActorBeginOverlap
  (params (OtherActor :type Actor%20Object%20Reference)))

(event EventTick
  (params (DeltaSeconds :type Float%20%28single-precision%29)))

(fn ConstructionScript)