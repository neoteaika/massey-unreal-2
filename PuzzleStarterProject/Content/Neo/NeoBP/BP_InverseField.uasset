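; BP_InverseField is a switchable field actor with inverted logic, solid when off and passable when on.
; On disables collision, hides the mesh and shows BridgeFX, while Off reverses all three; both call their parent event and play the same sound.
; BeginPlay starts with collision enabled and both components visible, and UpdateState sets collision directly from the State variable.
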(event EventBeginPlay
  (Collision|SetActorEnableCollision self true)
  (Rendering|SetVisibility (Variables|Default|GetBridgeFX) true false)
  (Rendering|SetVisibility (Variables|Character|GetMesh) true false))

(event Collision|EventActorBeginOverlap
  (params (OtherActor :type Actor%20Object%20Reference)))

(event EventTick
  (params (DeltaSeconds :type Float%20%28single-precision%29)))

(event EventOn
  (bind _self self)
  (|CallParentFunction)
  (Collision|SetActorEnableCollision _self false)
  (Rendering|SetVisibility (Variables|Character|GetMesh) false false)
  (Rendering|SetVisibility (Variables|Default|GetBridgeFX) true false)
  (Audio|PlaySoundatLocation "/Game/Neo/NeoMusic/hbfx_rec1_11.hbfx_rec1_11" (Transformation|GetActorLocation _self) "0, 0, 0" 1.0 1.0 0.0 0 0 0 0))

(event EventOff
  (bind _self self)
  (|CallParentFunction)
  (Collision|SetActorEnableCollision _self true)
  (Rendering|SetVisibility (Variables|Character|GetMesh) true false)
  (Rendering|SetVisibility (Variables|Default|GetBridgeFX) false false)
  (Audio|PlaySoundatLocation "/Game/Neo/NeoMusic/hbfx_rec1_11.hbfx_rec1_11" (Transformation|GetActorLocation _self) "0, 0, 0" 1.0 1.0 0.0 0 0 0 0))

(event EventUpdateState
  (Collision|SetActorEnableCollision (Variables|Default|GetState)))

(fn ConstructionScript
  (|CallParentFunction))